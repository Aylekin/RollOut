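; Player character for a rolling-ball platformer, with jump and wall jump, coin counting, pause menu and game-over screen.
; Tick drives side-to-side movement (world X in puzzle mode), spins the mesh from horizontal velocity and regenerates Energy.
; A line trace finds walls for launch-based wall jumps.
; A dynamic material shows the startup power-up animation and Power level; zero Power disables input and triggers game over.
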(event `self.ReceiveBeginPlay`
  ;[1 1 1] First set material instance
  (bind _returnvalue (`KismetMaterialLibrary.CreateDynamicMaterialInstance` (`PrimitiveComponent.GetMaterial` (`self.PlayerMesh`) 0)))
  (set `self.Player_Material_Instance` _returnvalue)
  ;[1 1 1] Change the color of the player
  (`self.Enable/Disable input` false)
  (`self.Change_Player_Material_Color` "IsActive")
  (`KismetSystemLibrary.Delay` 0.5)
  (`self.Change_Player_Material_Color` "IsActive" 1.0)
  (bind (_direction _value) (`Timeline|Player Activation Timeline`)
    (:`Update`
      (`self.Change_Player_Material_Color` "Power" (`KismetMathLibrary.Lerp` 0.0 (`self.Power`) _value)))
    (:`Finished`
      (`self.Enable/Disable input` true))))

(event `self.ReceiveTick`
  (params (DeltaSeconds :type "Float (single-precision)"))
  (`self.Movement Update`)
  (`self.RotateBall`)
  (`self.Energy Damage` -25.0)
  (if (`self.IsDead`)
    (bind _returnvalue (`|CreateWidget` "/Game/Blueprints/UI/BP_GameOverMenu.BP_GameOverMenu_C"))
    (`UserWidget.AddToViewport` _returnvalue 0)
    (set `PlayerController.bShowMouseCursor` true (`GameplayStatics.GetPlayerController` 0))
    (`GameplayStatics.SetGamePaused` true)))

(event `Enable/Disable input`
  (params (Enable :type Boolean))
  (bind _returnvalue (`GameplayStatics.GetPlayerController` 0))
  ;[1 1 1] Enable/Disable Input
  (if Enable
    (`self.EnableInput` _returnvalue)
    (else
      (`self.DisableInput` _returnvalue))))

(event `Change_Player_Material_Color`
  (params (`Param Name` :type Name) (Value :type "Float (double-precision)"))
  ;[1 1 1] Change player material color
  (`MaterialInstanceDynamic.SetScalarParameterValue` (`self.Player_Material_Instance`) `Param Name` Value)
  (`PrimitiveComponent.SetMaterial` (`self.PlayerMesh`) 0 (`self.Player_Material_Instance`)))

(event `Movement Update`
  ;[1 1 1] Movement Update
  (if (`self.Puzzle_Mode`)
    (set `self.Move Direction` (`KismetMathLibrary.MakeVector` (`self.GetInputAxisValue`)))
    (else
      (set `self.Move Direction` (`KismetMathLibrary.Normal` (* (`self.GetActorForwardVector`) (`self.GetInputAxisValue`))))))
  (`self.AddMovementInput` (`KismetMathLibrary.Normal` (`self.Move Direction`))))

(event `RotateBall`
  ;[1 1 1] Rotate Ball
  (bind _output_get (set `self.Flat Velocity` (`KismetMathLibrary.MakeVector` (.x (`self.GetVelocity`)) (.y (`self.GetVelocity`)))))
  (set `self.Current Speed` (`KismetMathLibrary.VSize` _output_get))
  (if (!= (`self.Current Speed`) 0.0)
    (set `self.Rotation Amount` (+ (`self.Rotation Amount`) (* (/ (`KismetMathLibrary.VSize` (`self.Flat Velocity`)) (* (`KismetMathLibrary.GetPI`) (`self.Ball Rotation Rate`))) (`GameplayStatics.GetWorldDeltaSeconds`))))
    (`SceneComponent.K2_SetWorldRotation` (`self.PlayerMesh`) (`KismetMathLibrary.RotatorFromAxisAndAngle` (`KismetMathLibrary.GetRightVector` (`KismetMathLibrary.MakeRotFromX` (`self.Flat Velocity`))) (`self.Rotation Amount`)) false false)))

(event `InputAction|Jump`
  (params (Key :type "Key Structure"))
  (bind _returnvalue (`self.GetActorForwardVector`))
  (bind _returnvalue_x (`KismetMathLibrary.BreakVector` (`self.K2_GetActorLocation`)))
  ;[1 1 1] Player Jump And Wall Jump
  (:`Pressed`
    (if (`NavMovementComponent.IsFalling` (`self.CharacterMovement`))
      (bind (_outhit _returnvalue_2) (`KismetSystemLibrary.LineTraceSingle` (- (`self.K2_GetActorLocation`) (* _returnvalue (+ (`CapsuleComponent.GetScaledCapsuleRadius` (`self.CapsuleComponent`)) 10.0))) (+ (`self.K2_GetActorLocation`) (* _returnvalue (+ (`CapsuleComponent.GetScaledCapsuleRadius` (`self.CapsuleComponent`)) 10.0))) "TraceTypeQuery1"))
      (if _returnvalue_2
        (`self.LaunchCharacter` (`KismetMathLibrary.MakeVector` (* (`KismetMathLibrary.SignOfFloat` (- _returnvalue_x (.x (`.Location` (`GameplayStatics.BreakHitResult` _outhit))))) 800.0) 0.0 1400.0) true true))
      (else
        (`self.Jump`)))))

(event `Power Damage`
  (params (Damage :type "Float (double-precision)"))
  ;[1 1 1] Power Damage
  (set `self.Power` (`KismetMathLibrary.FClamp` (- (`self.Power`) (* Damage (`GameplayStatics.GetWorldDeltaSeconds`))) 0.0 100.0))
  (`self.Change_Player_Material_Color` "Power" (`self.Power`))
  (if (<= (`self.Power`) 0.0)
    (set `self.IsDead` true)
    (`self.Change_Player_Material_Color` "IsOn")
    (`self.Enable/Disable input` false)))

(event `Energy Damage`
  (params (Damage :type "Float (double-precision)"))
  ;[1 1 1] Energy damage ( Positive values = damage, negative values = heal)
  (set `self.Energy` (`KismetMathLibrary.FClamp` (- (`self.Energy`) (* Damage (`GameplayStatics.GetWorldDeltaSeconds`) 1.0)) 0.0 100.0)))

(event `InputAction|Pause`
  (params (Key :type "Key Structure"))
  ;[1 1 1] Pause the game
  (:`Pressed`
    (`self.PauseGame`)))

(event `InputAction|ResetPosition`
  (params (Key :type "Key Structure"))
  (bind (_returnvalue_x _returnvalue_y _returnvalue_z) (`KismetMathLibrary.BreakVector` (`SceneComponent.K2_GetComponentLocation` (`self.PlayerMesh`))))
  (:`Pressed`
    (`self.K2_SetActorLocation` (`KismetMathLibrary.MakeVector` _returnvalue_x 0.0 _returnvalue_z))))

(event `AddCoin`
  (params (Coin :type Integer))
  (set `self.CoinsPoints` (+ (`self.CoinsPoints`) 1)))

(fn `PauseGame`
  (`GameplayStatics.SetGamePaused` true)
  (`/Engine/EditorBlueprintResources/StandardMacros.IsValid` (`self.PauseMenu`)
    (:`Is Valid`
      _)
    (:`Is Not Valid`
      (bind _returnvalue (`|CreateWidget` "/Game/Blueprints/UI/BP_PauseMenu.BP_PauseMenu_C" (`GameplayStatics.GetPlayerController` 0)))
      (set `self.PauseMenu` _returnvalue)))
  (`UserWidget.AddToViewport` (`self.PauseMenu`) 0)
  (`WidgetBlueprintLibrary.SetInputMode_UIOnlyEx` (`GameplayStatics.GetPlayerController` 0) (`self.PauseMenu`))
  (set `PlayerController.bShowMouseCursor` true (`GameplayStatics.GetPlayerController` 0)))

(fn `UnpauseGame`
  (`GameplayStatics.SetGamePaused` false)
  (`WidgetBlueprintLibrary.SetInputMode_GameOnly` (`GameplayStatics.GetPlayerController` 0))
  (set `PlayerController.bShowMouseCursor` false (`GameplayStatics.GetPlayerController` 0)))

(fn `UserConstructionScript`)