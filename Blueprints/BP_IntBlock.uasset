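; BP_IntBlock is an interactable physics cube that the player pulls toward themselves while holding the Action input inside its detection trigger.
; The trigger toggles input and the HUD prompt, and a physics constraint has all rotations locked after a delayed BeginPlay.
; A gated Tick drains player energy, updates the beam and applies mass-scaled horizontal force until release, low energy or an invalid player.
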(event `LockAllRotations`
  (bind _physicsconstraint (`self.PhysicsConstraint`))
  ;[1 1 1] Lock All Rotations Of Object
  (`PhysicsConstraintComponent.SetAngularSwing1Limit` _physicsconstraint "ACM_Locked" 0.0)
  (`PhysicsConstraintComponent.SetAngularSwing2Limit` _physicsconstraint "ACM_Locked" 0.0)
  (`PhysicsConstraintComponent.SetAngularTwistLimit` _physicsconstraint "ACM_Locked" 0.0))

(event `self.ReceiveBeginPlay`
  ;[1 1 1] Initialize the cube
  (`KismetSystemLibrary.Delay` 1.0) ; Delay because we want to give program a time to create HUD and REF to it
  (bind _asbp_player (cast `/Game/Blueprints/Bp_Player` (`GameplayStatics.GetPlayerPawn` 0)))
  (set `self.Player REF` _asbp_player)
  (set `self.UI HUD` (`/Game/Blueprints/Bp_Player.HUD REF` _asbp_player))
  (`self.LockAllRotations`)
  (`ActorComponent.Deactivate` (`self.Beam`)))

(event `self.Detection Trigger.OnComponentBeginOverlap`
  (params (OverlappedComponent :type "PrimitiveComponent Object Reference") (OtherActor :type "Actor Object Reference") (OtherComp :type "PrimitiveComponent Object Reference") (OtherBodyIndex :type Integer) (bFromSweep :type Boolean) (SweepResult :type "HitResult Structure (by ref)"))
  ;[1 1 1] Detecting collision with player
  (cast `/Game/Blueprints/Bp_Player` OtherActor)
  (`self.EnableInput` (`GameplayStatics.GetPlayerController` 0))
  (`/Game/Blueprints/UI/BP_GameHUD.Show InteractText` (`self.UI HUD`)))

(event `self.Detection Trigger.OnComponentEndOverlap`
  (params (OverlappedComponent :type "PrimitiveComponent Object Reference") (OtherActor :type "Actor Object Reference") (OtherComp :type "PrimitiveComponent Object Reference") (OtherBodyIndex :type Integer))
  ;[1 1 1] Detecting collision with player
  (cast `/Game/Blueprints/Bp_Player` OtherActor)
  (`self.DisableInput` (`GameplayStatics.GetPlayerController` 0))
  (`/Game/Blueprints/UI/BP_GameHUD.Hide InteractText` (`self.UI HUD`)))

(event `self.ReceiveTick`
  (params (DeltaSeconds :type "Float (single-precision)"))
  (bind _player_ref (`self.Player REF`))
  (bind (_returnvalue_x _returnvalue_y) (`KismetMathLibrary.BreakVector` (- (`self.K2_GetActorLocation` (`self.Player REF`)) (`SceneComponent.K2_GetComponentLocation` (`self.Mesh`)))))
  ;[1 1 1] Pull cube to the ball
  (`/Engine/EditorBlueprintResources/StandardMacros.Gate` true :!label _label
    (:`Exit`
      (`/Engine/EditorBlueprintResources/StandardMacros.IsValid` (`self.Player REF`) ; If player is dead then deactivate interaction
        (:`Is Valid`
          (`|ExecutionSequence`
            (:`then_0`
              (`/Game/Blueprints/Bp_Player.Energy Damage` _player_ref 50.0)
              (`ParticleSystemComponent.SetBeamSourcePoint` (`self.Beam`) 0 (`self.K2_GetActorLocation` _player_ref) 0)
              (`ParticleSystemComponent.SetBeamTargetPoint` (`self.Beam`) 0 (`SceneComponent.K2_GetComponentLocation` (`self.Mesh`)) 0))
            (:`then_1`
              (`/Engine/EditorBlueprintResources/StandardMacros.CompareFloat` (`/Game/Blueprints/Bp_Player.Energy` (`self.Player REF`)) 0.5 ; If 0 energy then don't interact
                (:`>`
                  (`PrimitiveComponent.AddForce` (`self.Mesh`) (* (`KismetMathLibrary.Normal` (`KismetMathLibrary.MakeVector` _returnvalue_x _returnvalue_y)) (* (`PrimitiveComponent.GetMass` (`self.Mesh`)) 1000.0)) "None" false))
                (:`==`
                  (`self.Close Interaction Gate` :!label _label_2)
                  (`/Game/Blueprints/UI/BP_GameHUD.Hide InteractText` (`self.UI HUD`)))
                (:`<`
                  (goto _label_2))))))
        (:`Is Not Valid`
          (`self.Close Interaction Gate`)
          (`/Game/Blueprints/UI/BP_GameHUD.Hide InteractText` (`self.UI HUD`)))))))

(event `InputAction|Action`
  (params (Key :type "Key Structure"))
  (bind _beam (`self.Beam`))
  ;[1 1 1] Pull cube to the ball
  (:`Pressed`
    (`ActorComponent.Activate` _beam true)
    (goto _label :!via `Open`))
  (:`Released`
    (`ActorComponent.Deactivate` _beam :!label _label_3)
    (goto _label :!via `Close`)))

(event `Close Interaction Gate`
  ;[1 1 1] Pull cube to the ball
  (goto _label_3))

(fn `UserConstructionScript`)